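; Hex grid manager that spawns BP_GridTile actors in an offset layout and holds the beginnings of A* pathfinding between tiles.
; SpawnTiles fills a coordinate-keyed TileMap, then AssignNeighbour links six neighbours per tile using column-parity offsets.
; FindDistanceBetweenTiles scores the start tile and its neighbours via SetMovementCosts, using a Manhattan heuristic on grid coordinates and updating tile visuals.
; The search is unfinished: TraverseForward is never called and its neighbour loop is empty.
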(event `self.SpawnTiles`
  (for _index (range 1 (+ (`KismetMathLibrary.FTrunc` (`.Y` (`KismetMathLibrary.BreakVector2D` (`self.GridSize`)))) 1))
    (for _index_2 (range 1 (+ (`KismetMathLibrary.FTrunc` (`KismetMathLibrary.BreakVector2D` (`self.GridSize`))) 1))
      (bind _returnvalue (`KismetMathLibrary.MakeVector2D` (`KismetMathLibrary.Conv_IntToDouble` _index) (`KismetMathLibrary.Conv_IntToDouble` _index_2)))
      (bind _returnvalue_2 (`self.GetSpawnTransform` _returnvalue))
      (bind _returnvalue_3 (`|SpawnActorFromClass` "/Game/_TableTop/Blueprints/World/BP_GridTile.BP_GridTile_C" _returnvalue_2 "AlwaysSpawn" "MultiplyWithRoot" null _returnvalue 1 null))
      (`BlueprintMapLibrary.Map_Add` (`self.TileMap`) _returnvalue _returnvalue_3)))
  (`self.AssignNeighbour`))

(event `self.FindDistanceBetweenTiles`
  (bind _value (`BlueprintMapLibrary.Map_Find` (`self.TileMap`) (`self.StartTileCoords`)))
  (`self.SetMovementCosts` _value (`self.MovementDoneTillNow`))
  (`KismetArrayLibrary.Array_Add` (`self.ClosedList`) _value)
  (for _array_element (`C_TileBase.Neighbours` _value)
    (`/Engine/EditorBlueprintResources/StandardMacros.IsValid` _array_element
      (:`Is Valid`
        (`KismetArrayLibrary.Array_Add` (`self.OpenList`) _array_element)
        (`self.SetMovementCosts` _array_element (`self.MovementDoneTillNow`))))))

(fn `AssignNeighbour`
  (locals (ThisTile :type "C_TileBase Object Reference"))
  (bind _coordinates_x (`KismetMathLibrary.BreakVector2D` (`C_TileBase.Coordinates` (`local.ThisTile`))))
  (bind _values (`BlueprintMapLibrary.Map_Values` (`self.TileMap`)))
  (for _array_element _values
    (set `local.ThisTile` _array_element)
    (for _index (range 6)
      (`KismetArrayLibrary.Array_Set` (`C_TileBase.Neighbours` (`local.ThisTile`)) _index (`BlueprintMapLibrary.Map_Find` (`self.TileMap`) (+ (`C_TileBase.Coordinates` (`local.ThisTile`)) (select `bool` (== (mod _coordinates_x 2.0) 0.0) :`false` (select `int` _index :`0` (-1.0 0.0) :`1` (0.0 1.0) :`2` (1.0 0.0) :`3` (1.0 -1.0) :`4` (0.0 -1.0) :`5` (-1.0 -1.0) :!type "Vector2D Structure") :`true` (select `int` _index :`0` (-1.0 1.0) :`1` (0.0 1.0) :`2` (1.0 1.0) :`3` (1.0 0.0) :`4` (0.0 -1.0) :`5` (-1.0 0.0) :!type "Vector2D Structure")))) true)))
  (return))

(fn `GetSpawnTransform`
  (params (Coords :type "Vector2D Structure"))
  (returns (ReturnValue :type "Transform Structure"))
  (bind _returnvalue_x (`KismetMathLibrary.BreakVector` (`self.K2_GetActorLocation`)))
  (bind _returnvalue (`self.GetTransform`))
  (bind (_returnvalue_x_2 _returnvalue_y) (`KismetMathLibrary.BreakVector` (`self.K2_GetActorLocation`)))
  (return (`KismetMathLibrary.MakeTransform` (`KismetMathLibrary.MakeVector` (+ (+ (* (`KismetMathLibrary.FTrunc` (`.Y` (`KismetMathLibrary.BreakVector2D` (`local.Coords`)))) (`self.HexagonInRadius`) 2.0) (`KismetMathLibrary.SelectFloat` (* (`self.HexagonInRadius`) -1.0) 0.0 (== (mod (`KismetMathLibrary.FTrunc` (`KismetMathLibrary.BreakVector2D` (`local.Coords`))) 2) 1))) _returnvalue_x) (+ (* (`KismetMathLibrary.FTrunc` (`KismetMathLibrary.BreakVector2D` (`local.Coords`))) (/ (* (`self.HexagonInRadius`) 2.0) (`KismetMathLibrary.Sqrt` 3.0)) 1.5) _returnvalue_y) (.z (.location _returnvalue))) (.rotation _returnvalue) (.scale _returnvalue))))

(fn `SetMovementCosts`
  (params (InThisTile :type "C_TileBase Object Reference (by ref)") (CurrentMovementCost :type Integer))
  (returns (Found :type Boolean))
  (bind (_coordinates_x _coordinates_y) (`KismetMathLibrary.BreakVector2D` (`C_TileBase.Coordinates` (`local.InThisTile`))))
  (bind (_coordinates_x_2 _coordinates_y_2) (`KismetMathLibrary.BreakVector2D` (`C_TileBase.Coordinates` (`BlueprintMapLibrary.Map_Find` (`self.TileMap`) (`self.EndTileCoords`)))))
  (bind _asbp_grid_tile (cast `/Game/_TableTop/Blueprints/World/BP_GridTile` (`local.InThisTile`)))
  (`/Game/_TableTop/Blueprints/World/BP_GridTile.ChangeColor` _asbp_grid_tile)
  (if (== (`local.InThisTile`) (`BlueprintMapLibrary.Map_Find` (`self.TileMap`) (`self.EndTileCoords`)))
    (return true)
    (else
      (set `C_TileBase.MovementCostToReachThisTile` (`KismetMathLibrary.SelectInt` 0 (+ (`C_TileBase.MovementCost` (`local.InThisTile`)) (`local.CurrentMovementCost`)) (`KismetMathLibrary.EqualExactly_Vector2DVector2D` (`C_TileBase.Coordinates` (`local.InThisTile`)) (`self.StartTileCoords`))) (`local.InThisTile`))
      (set `C_TileBase.MovementCostToReachTarget` (+ (`KismetMathLibrary.Abs_Int` (`KismetMathLibrary.FTrunc` (- _coordinates_x _coordinates_x_2))) (`KismetMathLibrary.Abs_Int` (`KismetMathLibrary.FTrunc` (- _coordinates_y _coordinates_y_2)))) (`local.InThisTile`))
      (set `C_TileBase.MovementCostTotal` (+ (`C_TileBase.MovementCostToReachThisTile` (`local.InThisTile`)) (`C_TileBase.MovementCostToReachTarget` (`local.InThisTile`))) (`local.InThisTile`))
      (set `self.MovementDoneTillNow` (+ (`C_TileBase.MovementCost` (`local.InThisTile`)) (`self.MovementDoneTillNow`)))
      (bind _asbp_grid_tile_2 (cast `/Game/_TableTop/Blueprints/World/BP_GridTile` (`local.InThisTile`)))
      (`/Game/_TableTop/Blueprints/World/BP_GridTile.SetValues` _asbp_grid_tile_2)
      (return false))))

(fn `TraverseForward`
  (params (InThisTile :type "C_TileBase Object Reference (by ref)"))
  (`KismetArrayLibrary.Array_RemoveItem` (`self.OpenList`) InThisTile)
  (if (not (== (`local.InThisTile`) (`BlueprintMapLibrary.Map_Find` (`self.TileMap`) (`self.EndTileCoords`))))
    (for _array_element (`C_TileBase.Neighbours` (`local.InThisTile`))
      (if (and (`KismetSystemLibrary.IsValid` _array_element) (not (`KismetArrayLibrary.Array_Contains` (`self.ClosedList`) _array_element)))
        _))))

(fn `UserConstructionScript`)