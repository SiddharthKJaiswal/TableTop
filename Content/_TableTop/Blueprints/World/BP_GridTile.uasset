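; BP_GridTile is a tabletop grid tile that displays its coordinates and pathfinding costs as text.
; The construction script writes the tile's Coordinates to a text label.
; SetValues writes the movement cost to reach the tile, the cost to the target and their total to G, H and F labels, matching A* notation.
; ChangeColor sets the tile mesh's material to M_Tile.
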(event `ChangeColor`
  (`PrimitiveComponent.SetMaterial` (`self.MeshComponent`) 0 "/Game/_TableTop/Assets/M_Tile.M_Tile"))

(event `SetValues`
  (`TextRenderComponent.K2_SetText` (`self.G`) (`KismetTextLibrary.Conv_IntToText` (`self.MovementCostToReachThisTile`)))
  (`TextRenderComponent.K2_SetText` (`self.H`) (`KismetTextLibrary.Conv_IntToText` (`self.MovementCostToReachTarget`)))
  (`TextRenderComponent.K2_SetText` (`self.F`) (`KismetTextLibrary.Conv_IntToText` (`self.MovementCostTotal`))))

(fn `UserConstructionScript`
  (`TextRenderComponent.K2_SetText` (`self.Coords`) (`KismetTextLibrary.Conv_Vector2dToText` (`self.Coordinates`))))